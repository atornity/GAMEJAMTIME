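; Base enemy Character that chases the player, takes damage with knockback, and dies at zero health.
; Any damage lowers Health, prints red debug messages, and destroys the actor when depleted.
; Point damage launches the character along the negated ShotFromDirection, overriding its velocity.
; While FollowPlayer is set, Tick feeds movement input straight toward the first player's character, without pathfinding.
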(event Game|Damage|EventAnyDamage
  (params (Damage :type Float%20%28single-precision%29) (DamageType :type Damage%20Type%20Object%20Reference) (InstigatedBy :type Controller%20Object%20Reference) (DamageCauser :type Actor%20Object%20Reference))
  ;[1 1 1] deal damage (any damage)
  (Development|PrintString (Utilities|String|Append "DEALT " (Utilities|String|ToString(Float) Damage) " DAMAGE") true true "(R=1.000000,G=0.000000,B=0.028412,A=1.000000)")
  (bind _output_get (Variables|Default|SetHealth (- (Variables|Default|GetHealth) Damage)))
  (Development|PrintString (Utilities|String|Append "HAS " (Utilities|String|ToString(Float) _output_get) " HEALTH") true true "(R=1.000000,G=0.000000,B=0.028412,A=1.000000)")
  (if (<= (Variables|Default|GetHealth) 0.0)
    (Development|PrintString "DEATH! I'M DEAD" true true "(R=1.000000,G=0.000000,B=0.028412,A=1.000000)")
    (Actor|DestroyActor)))

(event Game|Damage|EventPointDamage
  (params (Damage :type Float%20%28single-precision%29) (DamageType :type Damage%20Type%20Object%20Reference) (HitLocation :type Vector :default "0, 0, 0") (HitNormal :type Vector :default "0, 0, 0") (HitComponent :type Primitive%20Component%20Object%20Reference) (BoneName :type Name :default "None") (ShotFromDirection :type Vector :default "0, 0, 0") (InstigatedBy :type Controller%20Object%20Reference) (DamageCauser :type Actor%20Object%20Reference) (HitInfo :type Hit%20Result%20Structure%20%28by%20ref%29))
  ;[1 1 1] knockback
  (Character|LaunchCharacter (* ShotFromDirection -1e+02) true true))

(event EventTick
  (params (DeltaSeconds :type Float%20%28single-precision%29))
  ;[1 1 1] follow player character
  (if (Variables|Default|GetFollowPlayer)
    (Pawn|Input|AddMovementInput (Math|Vector|GetUnitDirection(Vector) (Transformation|GetActorLocation) (Transformation|GetActorLocation (Game|GetPlayerCharacter 0))) 1.0 false)))

(fn ConstructionScript)